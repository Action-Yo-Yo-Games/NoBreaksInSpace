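; BP_AI_SegwayCop is a Segway cop character that turns into a barricade cop when a car reaches it.
; Tick sets a very high max walk speed, slightly lower while the cop was recently rendered and higher when it is off screen.
; When its Box overlaps a BP_Car, it spawns a BP_BarricadeCop at its own transform, stores it as Wall, and destroys itself.
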(event OnComponentBeginOverlap(Box)
  (params (OverlappedComponent :type Primitive%20Component%20Object%20Reference) (OtherActor :type Actor%20Object%20Reference) (OtherComp :type Primitive%20Component%20Object%20Reference) (OtherBodyIndex :type Integer) (bFromSweep :type Boolean) (SweepResult :type Hit%20Result%20Structure%20%28by%20ref%29))
  (Utilities|Casting|CastToBP_Car OtherActor)
  (bind _returnvalue (Game|SpawnActorfromClass "/Game/Blueprints/AI/BP_BarricadeCop.BP_BarricadeCop_C" (Math|Transform|MakeTransform (Transformation|GetActorLocation) (Transformation|GetActorRotation) (Transformation|GetActorScale3D)) "AlwaysSpawn" "MultiplyWithRoot" 0 0))
  (Variables|Default|Setwall _returnvalue)
  (Actor|DestroyActor))

(event EventTick
  (params (DeltaSeconds :type Float%20%28single-precision%29))
  (bind _charactermovement (Variables|Character|GetCharacterMovement))
  (if (Class|Actor|WasRecentlyRendered 0.2)
    (Variables|/Script/Engine.CharacterMovementComponent|SetMaxWalkSpeed _charactermovement 5.9e+04)
    (else
      (Variables|/Script/Engine.CharacterMovementComponent|SetMaxWalkSpeed _charactermovement 6.1e+04))))

(fn ConstructionScript)