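; BP_DesertRaider is a desert raider actor that moves its character along a spline and is destroyed when something overlaps its box.
; Each tick advances a distance by spline speed and sets the character's relative transform from the spline in local space, with fixed height and yaw offsets.
; When looping is enabled, the distance resets to zero past the spline's end.
; Any overlap with the box destroys the whole actor.
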(event OnComponentBeginOverlap(Box)
  (params (OverlappedComponent :type Primitive%20Component%20Object%20Reference) (OtherActor :type Actor%20Object%20Reference) (OtherComp :type Primitive%20Component%20Object%20Reference) (OtherBodyIndex :type Integer) (bFromSweep :type Boolean) (SweepResult :type Hit%20Result%20Structure%20%28by%20ref%29))
  (Actor|DestroyActor))

(event EventTick
  (params (DeltaSeconds :type Float%20%28single-precision%29))
  (Variables|Default|SetDistanceAlongSpline (+ (* DeltaSeconds (Variables|Default|GetSplineSpeed)) (Variables|Default|GetDistanceAlongSpline)))
  (Transformation|SetRelativeTransform (Variables|Default|GetCharacter) (Math|Transform|MakeTransform (Math|Vector|MakeVector (.x (.location (Spline|GetTransformatDistanceAlongSpline (Variables|Default|GetSpline) (Variables|Default|GetDistanceAlongSpline) "Local" false))) (.y (.location (Spline|GetTransformatDistanceAlongSpline (Variables|Default|GetSpline) (Variables|Default|GetDistanceAlongSpline) "Local" false))) (+ (.z (.location (Spline|GetTransformatDistanceAlongSpline (Variables|Default|GetSpline) (Variables|Default|GetDistanceAlongSpline) "Local" false))) -89.0)) (Math|Rotator|MakeRotator (.roll (.rotation (Spline|GetTransformatDistanceAlongSpline (Variables|Default|GetSpline) (Variables|Default|GetDistanceAlongSpline) "Local" false))) (.pitch (.rotation (Spline|GetTransformatDistanceAlongSpline (Variables|Default|GetSpline) (Variables|Default|GetDistanceAlongSpline) "Local" false))) (+ (.yaw (.rotation (Spline|GetTransformatDistanceAlongSpline (Variables|Default|GetSpline) (Variables|Default|GetDistanceAlongSpline) "Local" false))) -9e+01)) (Variables|/Script/Engine.SceneComponent|GetRelativeScale3D (Variables|Default|GetCharacter))) false false)
  (if (Variables|Default|GetLoop)
    (if (> (Variables|Default|GetDistanceAlongSpline) (Spline|GetSplineLength (Variables|Default|GetSpline)))
      (Variables|Default|SetDistanceAlongSpline 0.0))))

(fn ConstructionScript)