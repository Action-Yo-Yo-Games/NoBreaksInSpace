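; BP_EnemyBullet is an enemy projectile that temporarily slows any BP_Ship it overlaps.
; On a sphere overlap it caches the ship's max walk speed, subtracts a fixed penalty and prints the result.
; After a delay it restores the cached speed and destroys itself, so the bullet actor must outlive the slow effect.
; A lifespan set at BeginPlay also removes the bullet, which can preempt the restore on late hits.
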(event OnComponentBeginOverlap(Sphere)
  (params (OverlappedComponent :type Primitive%20Component%20Object%20Reference) (OtherActor :type Actor%20Object%20Reference) (OtherComp :type Primitive%20Component%20Object%20Reference) (OtherBodyIndex :type Integer) (bFromSweep :type Boolean) (SweepResult :type Hit%20Result%20Structure%20%28by%20ref%29))
  (bind _asbp_ship (Utilities|Casting|CastToBP_Ship OtherActor))
  (Variables|Default|SetOldSpeed (Variables|/Script/Engine.CharacterMovementComponent|GetMaxWalkSpeed (Variables|/Script/Engine.Character|GetCharacterMovement _asbp_ship)))
  (bind _output_get (Variables|/Script/Engine.CharacterMovementComponent|SetMaxWalkSpeed (Variables|/Script/Engine.Character|GetCharacterMovement _asbp_ship) (- (Variables|/Script/Engine.CharacterMovementComponent|GetMaxWalkSpeed (Variables|/Script/Engine.Character|GetCharacterMovement _asbp_ship)) 1e+03)))
  (Development|PrintString (Utilities|String|ToString(Float) _output_get))
  (Utilities|FlowControl|Delay 3.0)
  (Variables|/Script/Engine.CharacterMovementComponent|SetMaxWalkSpeed (Variables|/Script/Engine.Character|GetCharacterMovement _asbp_ship) (Variables|Default|GetOldSpeed))
  (Actor|DestroyActor))

(event EventBeginPlay
  (Actor|SetLifeSpan 1e+01))

(fn ConstructionScript)