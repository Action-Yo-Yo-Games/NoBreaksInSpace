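; BP_AI_SpaceCop is a stationary enemy that shoots at the player's ship.
; From BeginPlay, Shoot turns the actor and its BulletSpawner toward the ship, then spawns BP_EnemyBullet if within range.
; It re-calls itself after a random delay only when in range, so an out-of-range check ends firing permanently.
; Overlap of its capsule with a BP_Bullet destroys it with an explosion effect.
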(event OnComponentBeginOverlap(CapsuleComponent)
  (params (OverlappedComponent :type Primitive%20Component%20Object%20Reference) (OtherActor :type Actor%20Object%20Reference) (OtherComp :type Primitive%20Component%20Object%20Reference) (OtherBodyIndex :type Integer) (bFromSweep :type Boolean) (SweepResult :type Hit%20Result%20Structure%20%28by%20ref%29))
  (bind _returnvalue (Transformation|GetActorTransform))
  (Utilities|Casting|CastToBP_Bullet OtherActor)
  (Actor|DestroyActor)
  (Niagara|SpawnSystematLocation "/Game/Niagara/Explosion/FX_Explosion.FX_Explosion" (Transformation|GetActorLocation) (.rotation _returnvalue) (.scale _returnvalue)))

(event Custom|Shoot
  (CallFunction|FindPlayer)
  (bind _asbp_player_controller (Utilities|Casting|CastToBP_PlayerController (Game|Player|GetPlayerPawn 0)))
  (if (<= (Transformation|GetDistanceTo (Variables|/Game/Blueprints/Player/CarBP/BP_Car.BP_Car_C|GetShipReference (Variables|/Game/Blueprints/Player/BP_PlayerController.BP_PlayerController_C|GetCar _asbp_player_controller)) self) 5e+04)
    (Game|SpawnActorfromClass "/Game/Blueprints/AI/BP_EnemyBullet.BP_EnemyBullet_C" (Transformation|GetWorldTransform (Variables|Default|GetBulletSpawner)) "Undefined" "MultiplyWithRoot" 0 0)
    (Utilities|FlowControl|Delay (Math|Conversions|ToFloat(Integer) (Math|Random|RandomInteger 5)))
    (CallFunction|Shoot)))

(event Custom|Find%20Player
  (bind _asbp_player_controller (Utilities|Casting|CastToBP_PlayerController (Game|Player|GetPlayerPawn 0)))
  (Transformation|SetWorldTransform (Variables|Default|GetBulletSpawner) (Math|Transform|MakeTransform (Transformation|GetActorLocation) (Math|Rotator|FindLookatRotation (Transformation|GetActorLocation) (Transformation|GetActorLocation (Variables|/Game/Blueprints/Player/CarBP/BP_Car.BP_Car_C|GetShipReference (Variables|/Game/Blueprints/Player/BP_PlayerController.BP_PlayerController_C|GetCar _asbp_player_controller)))) "1.000000,1.000000,1.000000") false false)
  (Transformation|SetActorTransform (Math|Transform|MakeTransform (Transformation|GetActorLocation) (Math|Rotator|FindLookatRotation (Transformation|GetActorLocation) (Transformation|GetActorLocation (Variables|/Game/Blueprints/Player/CarBP/BP_Car.BP_Car_C|GetShipReference (Variables|/Game/Blueprints/Player/BP_PlayerController.BP_PlayerController_C|GetCar _asbp_player_controller)))) "1.000000,1.000000,1.000000")))

(event EventBeginPlay
  (CallFunction|Shoot))

(event Collision|EventActorBeginOverlap
  (params (OtherActor :type Actor%20Object%20Reference)))

(fn ConstructionScript)