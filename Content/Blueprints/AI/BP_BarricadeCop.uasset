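; BP_BarricadeCop is a placed stand-in cop that turns into an active AI segway cop when the player's car comes near.
; Tick casts the player pawn to BP_PlayerController and checks its Car's distance to this actor against a fixed range.
; Once in range, it waits briefly, spawns BP_AI_SegwayCop with BT_SegwayCop at its own location and rotation, then destroys itself.
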(event OnComponentHit(EnemyMesh)
  (params (HitComponent :type Primitive%20Component%20Object%20Reference) (OtherActor :type Actor%20Object%20Reference) (OtherComp :type Primitive%20Component%20Object%20Reference) (NormalImpulse :type Vector :default "0, 0, 0") (Hit :type Hit%20Result%20Structure%20%28by%20ref%29)))

(event EventTick
  (params (DeltaSeconds :type Float%20%28single-precision%29))
  (bind _returnvalue (Transformation|GetActorLocation))
  (bind _asbp_player_controller (Utilities|Casting|CastToBP_PlayerController (Game|Player|GetPlayerPawn 0)))
  (if (<= (Transformation|GetDistanceTo (Variables|/Game/Blueprints/Player/BP_PlayerController.BP_PlayerController_C|GetCar _asbp_player_controller) self) 7.09e+03)
    (Utilities|FlowControl|Delay 1.0)
    (AI|SpawnAIFromClass "/Game/Blueprints/AI/BP_AI_SegwayCop.BP_AI_SegwayCop_C" "/Game/Blueprints/AI/BT_SegwayCop.BT_SegwayCop" (Math|Vector|MakeVector (.x _returnvalue) (.y _returnvalue) (.z _returnvalue)) (Transformation|GetActorRotation) true 0)
    (Actor|DestroyActor)))

(event Collision|EventActorBeginOverlap
  (params (OtherActor :type Actor%20Object%20Reference)))

(event EventBeginPlay)

(fn ConstructionScript)