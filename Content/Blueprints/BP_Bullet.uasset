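; BP_Bullet is a projectile actor that flies at a constant speed and destroys itself five seconds after spawning.
; Tick moves it along the Arrow component's forward vector without sweeping, and no hit or overlap logic runs.
; BeginPlay halves the spawn yaw, which offsets the double rotation caused by feeding a world-space vector into AddActorLocalOffset.
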(event EventBeginPlay
  (bind _returnvalue (Transformation|GetActorRotation))
  (Transformation|SetActorRotation (Math|Rotator|MakeRotator (.roll _returnvalue) (.pitch _returnvalue) (/ (.yaw _returnvalue) 2.0)))
  (Utilities|FlowControl|Delay 5.0)
  (Actor|DestroyActor))

(event Collision|EventActorBeginOverlap
  (params (OtherActor :type Actor%20Object%20Reference)))

(event EventTick
  (params (DeltaSeconds :type Float%20%28single-precision%29))
  (Transformation|AddActorLocalOffset (* (Math|Vector|Normalize (Math|Vector|GetForwardVector (Variables|Default|GetArrow))) DeltaSeconds 5e+03) false false))

(fn ConstructionScript)