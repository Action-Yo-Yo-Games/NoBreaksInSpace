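; BP_Drive is a trigger actor that shows the P_Drive prompt widget while the player's car is inside its box.
; It constructs the widget once on BeginPlay and keeps it as PromptScreen.
; Box overlap events cast player pawn 0 to BP_PlayerController and compare the overlapping actor with its Car reference, adding the widget to the viewport on entry and removing it on exit.
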(event OnComponentBeginOverlap(Box)
  (params (OverlappedComponent :type Primitive%20Component%20Object%20Reference) (OtherActor :type Actor%20Object%20Reference) (OtherComp :type Primitive%20Component%20Object%20Reference) (OtherBodyIndex :type Integer) (bFromSweep :type Boolean) (SweepResult :type Hit%20Result%20Structure%20%28by%20ref%29))
  (bind _asbp_player_controller (Utilities|Casting|CastToBP_PlayerController (Game|Player|GetPlayerPawn 0)))
  (if (== OtherActor (Variables|/Game/Blueprints/Player/BP_PlayerController.BP_PlayerController_C|GetCar _asbp_player_controller))
    (UserInterface|Viewport|AddtoViewport (Variables|Default|GetPromptScreen) 0)))

(event OnComponentEndOverlap(Box)
  (params (OverlappedComponent :type Primitive%20Component%20Object%20Reference) (OtherActor :type Actor%20Object%20Reference) (OtherComp :type Primitive%20Component%20Object%20Reference) (OtherBodyIndex :type Integer))
  (bind _asbp_player_controller (Utilities|Casting|CastToBP_PlayerController (Game|Player|GetPlayerPawn 0)))
  (if (== OtherActor (Variables|/Game/Blueprints/Player/BP_PlayerController.BP_PlayerController_C|GetCar _asbp_player_controller))
    (Widget|RemovefromParent (Variables|Default|GetPromptScreen))))

(event EventBeginPlay
  (bind _returnvalue (Game|ConstructObjectfromClass "/Game/Blueprints/UI_Prompts/P_Drive.P_Drive_C"))
  (Variables|Default|SetPromptScreen _returnvalue))

(event Collision|EventActorBeginOverlap
  (params (OtherActor :type Actor%20Object%20Reference)))

(event EventTick
  (params (DeltaSeconds :type Float%20%28single-precision%29)))

(fn ConstructionScript)