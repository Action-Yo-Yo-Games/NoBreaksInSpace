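; Asteroid obstacle that spins and drifts, breaking down when shot and exploding on contact with a ship.
; SpawnWithParams sets its scale, spin and velocity through the rotating and floating pawn movement components.
; Each bullet overlap halves its scale and spawns an explosion, destroying it once small enough, otherwise granting brief invulnerability.
; Overlapping a ship spawns an explosion at the ship's mesh and destroys the asteroid itself.
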(event Custom|SpawnWithParams
  (params (Scale :type Vector) (Rotation%20Rate :type Rotator) (Velocity :type Vector))
  (Transformation|SetActorScale3D Scale)
  (Variables|/Script/Engine.RotatingMovementComponent|SetRotationRate (Variables|Default|GetRotatingMovement) Rotation%20Rate)
  (Variables|/Script/Engine.MovementComponent|SetVelocity (Variables|Default|GetFloatingPawnMovement) Velocity))

(event Collision|EventActorBeginOverlap
  (params (OtherActor :type Actor%20Object%20Reference))
  (bind _returnvalue (Transformation|GetActorTransform))
  (bind _returnvalue_2 (Transformation|GetActorTransform))
  (Variables|Default|SetActorLoc (Transformation|GetActorLocation OtherActor))
  (Utilities|FlowControl|Sequence
    (:then_0
      (if (and (Variables|Default|GetVulnerable) (== (Utilities|GetClass OtherActor) "/Game/Blueprints/BP_Bullet.BP_Bullet_C"))
        (Transformation|SetActorScale3D (/ (Transformation|GetActorScale3D) 2.0))
        (Variables|Default|SetVulnerable false)
        (Niagara|SpawnSystematLocation "/Game/Niagara/Explosion/FX_Explosion.FX_Explosion" (Variables|Default|GetActorLoc) (.rotation _returnvalue_2) (.scale _returnvalue_2))
        (if (< (Math|Vector|VectorLength (Transformation|GetActorScale3D)) 5.0)
          (Actor|DestroyActor)
          (else
            (Utilities|FlowControl|Delay 0.2)
            (Variables|Default|SetVulnerable true)))))
    (:then_1
      (bind _asbp_ship (Utilities|Casting|CastToBP_Ship OtherActor))
      (Niagara|SpawnSystematLocation "/Game/Niagara/Explosion/FX_Explosion.FX_Explosion" (Transformation|GetWorldLocation (Variables|/Script/Engine.Character|GetMesh _asbp_ship)) (.rotation _returnvalue) (.scale _returnvalue))
      (Actor|DestroyActor))))

(event EventTick
  (params (DeltaSeconds :type Float%20%28single-precision%29)))

(fn ConstructionScript)