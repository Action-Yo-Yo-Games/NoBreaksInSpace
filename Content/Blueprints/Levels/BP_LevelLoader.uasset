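; Level loader actor that spawns the test planet levels as level instances at runtime.
; On BeginPlay it fills a list of levels and loads each by soft object pointer, spacing them far apart along X.
; Disconnected logic would gather lighting, skybox and atmosphere references from BP_LevelData actors and copy the current level's light color and rotation to a shared light.
; The LoadLevelLighting event is empty.
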(event Custom|LoadLevelLighting)

(event EventBeginPlay
  (bind _levelstoload (Variables|Default|GetLevelsToLoad))
  (Utilities|Array|Add _levelstoload "/Game/Blueprints/Levels/TestPlanet.TestPlanet")
  (Utilities|Array|Add _levelstoload "/Game/Blueprints/Levels/TestPlanet2.TestPlanet2")
  (for (_array_element _array_index) _levelstoload
    (Class|LevelStreamingDynamic|LoadLevelInstancebySoftObjectPtr _array_element (Math|Vector|MakeVector (* _array_index 5e+04) 0.0 0.0) "0, 0, 0" "" 0 false)))

(fn ConstructionScript)