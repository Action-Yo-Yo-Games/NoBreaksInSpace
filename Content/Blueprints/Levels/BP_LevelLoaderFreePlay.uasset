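; Free-play level loader that builds a long course along X from level instances chosen in the LevelSaver actor.
; On BeginPlay it queues the first level, repeats the middle three, appends the fifth, then streams each in at evenly spaced offsets.
; Each segment gets a row of asteroids, with stream-random offsets and scales and unseeded random spin.
; Older queueing and BP_LevelData lighting-collection logic remains disconnected.
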(event EventBeginPlay
  (bind _returnvalue (Math|Random|RandomRotator true))
  (bind _levelstoload (Variables|Default|GetLevelsToLoad))
  (bind _returnvalue_2 (Actor|GetActorOfClass "/Game/Blueprints/Levels/LevelSaver.LevelSaver_C"))
  (Math|Random|SetRandomStreamSeed (Variables|Default|GetStream) (Math|Random|RandomInteger 0))
  (Utilities|Array|Add _levelstoload (Variables|/Game/Blueprints/Levels/LevelSaver.LevelSaver_C|GetFirst%20Level _returnvalue_2))
  (for _index (range 0 3)
    (Utilities|Array|Add _levelstoload (Variables|/Game/Blueprints/Levels/LevelSaver.LevelSaver_C|GetSecond%20Level _returnvalue_2))
    (Utilities|Array|Add _levelstoload (Variables|/Game/Blueprints/Levels/LevelSaver.LevelSaver_C|GetThird%20Level _returnvalue_2))
    (Utilities|Array|Add _levelstoload (Variables|/Game/Blueprints/Levels/LevelSaver.LevelSaver_C|GetFourth%20Level _returnvalue_2)))
  (Utilities|Array|Add _levelstoload (Variables|/Game/Blueprints/Levels/LevelSaver.LevelSaver_C|GetFifth%20Level _returnvalue_2))
  (for (_array_element _array_index) _levelstoload
    (Class|LevelStreamingDynamic|LoadLevelInstancebySoftObjectPtr _array_element (Math|Vector|MakeVector (* _array_index 1e+05) 0.0 0.0) "0, 0, 0" "" 0 false)
    (for _index_2 (range 0 6)
      (bind _returnvalue_3 (Game|SpawnActorfromClass "/Game/Blueprints/Obstacles/BP_Asteroid.BP_Asteroid_C" (Math|Transform|MakeTransform (Math|Vector|MakeVector (+ (* _array_index 1e+05) (* _index_2 1e+03) 5e+04) (Math|Random|RandomFloatinRangefromStream (Variables|Default|GetStream) -4e+02 4e+02) (Math|Random|RandomFloatinRangefromStream (Variables|Default|GetStream) -4e+02 4e+02)) "0, 0, 0" "1.000000,1.000000,1.000000") "Undefined" "MultiplyWithRoot" 0 0))
      (Default|SpawnwithParams _returnvalue_3 (Math|Vector|MakeVector (Math|Random|RandomFloatinRangefromStream (Variables|Default|GetStream) 1e+01 15.0) (Math|Random|RandomFloatinRangefromStream (Variables|Default|GetStream) 1e+01 15.0) (Math|Random|RandomFloatinRangefromStream (Variables|Default|GetStream) 1e+01 15.0)) (Math|Rotator|MakeRotator (/ (.roll _returnvalue) 8.0) (/ (.pitch _returnvalue) 8.0) (/ (.yaw _returnvalue) 8.0)) "0, 0, 0"))))

(fn ConstructionScript)