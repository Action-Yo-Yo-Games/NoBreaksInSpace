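; BP_Ship is the player's flying ship Character, which constantly moves forward and swaps possession to a car on overlapping BP_SwapToCar or on debug input.
; Move input offsets the mesh within a radius around the actor and banks it, easing level on release.
; Shooting spawns rate-limited bullets and builds heat that locks fire until fully cooled, while boost multiplies forward and side speeds.
; Possession enables flying, collision and visibility; unpossession hides the ship.
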(event Input|EnhancedActionEvents|EnhancedInputActionIA_Shoot
  (params (ActionValue :type Boolean) (ElapsedSeconds :type Float%20%28double-precision%29) (TriggeredSeconds :type Float%20%28double-precision%29) (InputAction :type Input%20Action%20Object%20Reference :default "/Game/Blueprints/Player/ShipBP/IA_Shoot.IA_Shoot"))
  (bind _returnvalue (Actor|GetGameTimeSinceCreation))
  (:Triggered
    (if (and (>= (- _returnvalue (Variables|Default|GetPrevFireTime)) (Variables|Default|GetFireRate)) (not (Variables|Default|GetOverheated)))
      (Variables|Default|SetPrevFireTime _returnvalue)
      (Game|SpawnActorfromClass "/Game/Blueprints/BP_Bullet.BP_Bullet_C" (Transformation|GetActorTransform) "Undefined" 0 0)
      (Variables|Default|SetHeatup (Math|Float|Clamp(Float) (+ (Variables|Default|GetHeatupSpeed) (Variables|Default|GetHeatup)) 0.0 1e+02))
      (Variables|Default|SetIsShooting true)
      (if (>= (Variables|Default|GetHeatup) 1e+02)
        (Variables|Default|SetOverheated true)
        (Variables|Default|SetIsShooting false))))
  (:Completed
    (Variables|Default|SetIsShooting false)))

(event Input|EnhancedActionEvents|EnhancedInputActionIA_Move
  (params (ActionValue :type Vector%202D%20Structure) (ElapsedSeconds :type Float%20%28double-precision%29) (TriggeredSeconds :type Float%20%28double-precision%29) (InputAction :type Input%20Action%20Object%20Reference :default "/Game/Blueprints/Player/ShipBP/IA_Move.IA_Move"))
  (bind _mesh (Variables|Character|GetMesh))
  (bind _relativerotation (Variables|/Script/Engine.SceneComponent|GetRelativeRotation _mesh))
  (bind (_roll _pitch _yaw) (Math|Rotator|BreakRotator _relativerotation))
  (:Triggered
    (Class|SceneComponent|AddWorldTransform (Variables|Character|GetMesh) (Math|Transform|MakeTransform (* (+ (* (Transformation|GetActorRightVector) (.x ActionValue)) (* (.y ActionValue) (Transformation|GetActorUpVector))) (Variables|Default|GetSideSpeed)) "0, 0, 0" "1.000000,1.000000,1.000000") false false)
    (if (> (Math|Vector|VectorLength (Variables|/Script/Engine.SceneComponent|GetRelativeLocation (Variables|Character|GetMesh))) (Variables|Default|GetDistanceLimit))
      (Transformation|SetRelativeLocation (Variables|Character|GetMesh) (* (Math|Vector|Normalize (Variables|/Script/Engine.SceneComponent|GetRelativeLocation (Variables|Character|GetMesh))) (Variables|Default|GetDistanceLimit)) false false))
    (Transformation|SetRelativeRotation (Variables|Character|GetMesh) (Math|Interpolation|RInterpTo _relativerotation (Math|Rotator|MakeRotator (* (.x ActionValue) 6e+01) _pitch _yaw) (Utilities|Time|GetWorldDeltaSeconds) 1e+01) false false)
    (Variables|Default|SetisTurning true))
  (:Completed
    (Variables|Default|SetisTurning false)))

(event Input|EnhancedActionEvents|EnhancedInputActionIA_Boost
  (params (ActionValue :type Float%20%28double-precision%29) (ElapsedSeconds :type Float%20%28double-precision%29) (TriggeredSeconds :type Float%20%28double-precision%29) (InputAction :type Input%20Action%20Object%20Reference :default "/Game/Blueprints/Player/ShipBP/IA_Boost.IA_Boost"))
  (bind _charactermovement (Variables|Character|GetCharacterMovement))
  (bind _charactermovement_2 (Variables|Character|GetCharacterMovement))
  (:Started
    (Variables|/Script/Engine.CharacterMovementComponent|SetMaxFlySpeed _charactermovement_2 (* (Variables|/Script/Engine.CharacterMovementComponent|GetMaxFlySpeed _charactermovement_2) (Variables|Default|GetBoostSpeedMultiplier)))
    (Variables|Default|SetSideSpeed (* (Variables|Default|GetSideSpeed) (Variables|Default|GetBoostSideSpeedMultiplier))))
  (:Completed
    (Variables|/Script/Engine.CharacterMovementComponent|SetMaxFlySpeed _charactermovement (/ (Variables|/Script/Engine.CharacterMovementComponent|GetMaxFlySpeed _charactermovement) (Variables|Default|GetBoostSpeedMultiplier)))
    (Variables|Default|SetSideSpeed (/ (Variables|Default|GetSideSpeed) (Variables|Default|GetBoostSideSpeedMultiplier)))))

(event Input|EnhancedActionEvents|EnhancedInputActionIA_DEBUG_Swap
  (params (ActionValue :type Boolean) (ElapsedSeconds :type Float%20%28double-precision%29) (TriggeredSeconds :type Float%20%28double-precision%29) (InputAction :type Input%20Action%20Object%20Reference :default "/Game/Blueprints/Player/IA_DEBUG_Swap.IA_DEBUG_Swap"))
  (bind _carreference (Variables|Default|GetCarReference))
  (:Triggered
    (Utilities|IsValid _carreference
      (:Is%20Valid
        (Input|DisableInput 0)
        (Transformation|SetActorTransform _carreference (Transformation|GetActorTransform))
        (Components|MoveComponentTo (Variables|Character|GetMesh) "0, 0, 0" "0, 0, 0" false false 1.0 false)
        (Transformation|SetActorTransform _carreference (Transformation|GetActorTransform))
        (Pawn|Possess (Game|GetPlayerController 0) _carreference)))))

(event EventBeginPlay
  (bind _asplayer_controller (Utilities|Casting|CastToPlayerController (Pawn|GetController)))
  (Utilities|IsValid (PlayerController|LocalPlayerSubsystems|GetEnhancedInputLocalPlayerSubsystem _asplayer_controller)
    (:Is%20Valid
      (Input|AddMappingContext (PlayerController|LocalPlayerSubsystems|GetEnhancedInputLocalPlayerSubsystem _asplayer_controller) "/Game/Blueprints/Player/IMC_Player.IMC_Player" 0 "(bIgnoreAllPressedKeysUntilRelease=True,bForceImmediately=False)"))))

(event EventUnpossessed
  (params (OldController :type Controller%20Object%20Reference))
  (Collision|SetActorEnableCollision false)
  (Rendering|SetActorHiddenInGame true))

(event EventTick
  (params (DeltaSeconds :type Float%20%28single-precision%29))
  (Utilities|FlowControl|Sequence
    (:then_0
      (if (not (Variables|Default|GetIsShooting))
        (bind _output_get (Variables|Default|SetHeatup (Math|Float|Clamp(Float) (- (Variables|Default|GetHeatup) (* (Variables|Default|GetCooldownSpeed) DeltaSeconds)) 0.0 1e+02)))
        ;[1 1 1] Replace Print With UI Updates
        (Development|PrintString (Utilities|String|ToString(Float) _output_get))
        (if (== (Variables|Default|GetHeatup) 0.0)
          (Variables|Default|SetOverheated false))))
    (:then_1
      (if true
        (Pawn|Input|AddMovementInput (Transformation|GetActorForwardVector) 1e+03 false)
        (if (not (Variables|Default|GetisTurning))
          (Transformation|SetRelativeRotation (Variables|Character|GetMesh) (Math|Interpolation|RInterpTo (Variables|/Script/Engine.SceneComponent|GetRelativeRotation (Variables|Character|GetMesh)) (Math|Rotator|MakeRotator 0.0 0.0 0.0) (Utilities|Time|GetWorldDeltaSeconds) 1e+01) false false))))))

(event Collision|EventActorBeginOverlap
  (params (OtherActor :type Actor%20Object%20Reference))
  (bind _carreference (Variables|Default|GetCarReference))
  (if (== (Utilities|GetClass OtherActor) "/Game/Blueprints/BP_SwapToCar.BP_SwapToCar_C")
    (Transformation|SetActorRotation (Transformation|GetActorRotation OtherActor))
    (Utilities|IsValid _carreference
      (:Is%20Valid
        (Input|DisableInput 0)
        (Transformation|SetActorTransform _carreference (Transformation|GetActorTransform))
        (Components|MoveComponentTo (Variables|Character|GetMesh) "0, 0, 0" "0, 0, 0" false false 1.0 false)
        (Transformation|SetActorTransform _carreference (Transformation|GetActorTransform))
        (Pawn|Possess (Game|GetPlayerController 0) _carreference)))))

(event EventPossessed
  (params (NewController :type Controller%20Object%20Reference))
  (Collision|SetActorEnableCollision true)
  (Rendering|SetActorHiddenInGame false)
  (Variables|/Script/Engine.CharacterMovementComponent|SetMaxFlySpeed (Variables|Character|GetCharacterMovement) (Variables|Default|GetBaseForwardSpeed))
  (Input|EnableInput 0)
  (Pawn|Components|CharacterMovement|SetMovementMode (Variables|Character|GetCharacterMovement) "MOVE_Flying" 0))

(fn ConstructionScript)