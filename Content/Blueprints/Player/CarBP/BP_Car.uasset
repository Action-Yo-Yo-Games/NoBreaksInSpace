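; Player car built on CharacterMovement that drives, drifts with reduced friction, and can earn a startup boost.
; Input events adjust speed, yaw and camera, while Tick applies decaying speed as forward input, drives engine pitch and camera distance, and tilts meshes to turns and traced ground normals.
; Overlapping BP_SwapToPlane hands the transform and visibility to the referenced ship.
; SetCarType only configures type 0; other presets are unconnected.
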(event Custom|SetCarType
  (params (TypeID :type Integer) (PlayerID :type Integer))
  (Variables|Default|SetType%20ID TypeID)
  (Variables|Default|SetPlayer%20ID PlayerID)
  (Utilities|FlowControl|Sequence
    (:then_0
      (if (== (Variables|Default|GetType%20ID) 0)
        (Variables|Default|SetSpeedMultiplier 5.0)
        (Variables|Default|SetAcceleration 3e+01)
        (Variables|Default|SetDeceleration 1.0)
        (Variables|Default|SetTurnValue 2.0)
        (Variables|Default|SetFriction 8.0)
        (Variables|Default|SetHillSpeed 1.0)
        (Variables|Default|SetDriftMaxSpeedMultiplier 0.7)
        (Variables|Default|SetDriftTurnMultiplier 2.0)
        (Variables|Default|SetDriftFrictionMultiplier 0.125)
        (Variables|Default|SetStartupBoost 1.5)
        (Variables|Default|SetSecondsToBoost 0.3)
        (Development|SetHiddeninGame (Variables|Default|GetSM_SportsCar) false true)
        (Input|EnableInput 0)))))

(event Custom|Accelerate
  (params (ElapsedSeconds :type Float%20%28double-precision%29))
  (bind _returnvalue (Transformation|GetActorForwardVector))
  (bind _returnvalue_2 (Transformation|GetActorForwardVector))
  (bind _hillspeed (Variables|Default|GetHillSpeed))
  (bind _maxspeed (Variables|Default|GetMaxSpeed))
  (bind _maxspeed_2 (Variables|Default|GetMaxSpeed))
  (bind _mesh (Variables|Character|GetMesh))
  (bind _mesh_2 (Variables|Character|GetMesh))
  (bind _returnvalue_3 (Math|Vector|GetUpVector _mesh))
  (bind _returnvalue_4 (Math|Vector|GetUpVector _mesh_2))
  (bind _returnvalue_5 (Math|Vector|DotProduct _returnvalue _returnvalue_4))
  (bind _returnvalue_6 (Math|Vector|DotProduct _returnvalue_2 _returnvalue_3))
  (bind _returnvalue_7 (* _returnvalue_6 _hillspeed 1.0))
  (bind _returnvalue_8 (* _returnvalue_5 0.0 1.0))
  (bind _returnvalue_9 (- _maxspeed _returnvalue_8))
  (bind _returnvalue_10 (- _maxspeed_2 _returnvalue_7))
  (if (not (and (== (Variables|Default|GetCurrentSpeed) 0.0) (Variables|Default|GetIsDrifting)))
    (if (and (Variables|Default|GetIsTurning) (Variables|Default|GetIsDrifting))
      (if (< (Variables|Default|GetCurrentSpeed) (* _returnvalue_10 (Variables|Default|GetDriftMaxSpeedMultiplier)))
        (Variables|Default|SetCurrentSpeed (Math|Float|Clamp(Float) (+ (Variables|Default|GetCurrentSpeed) (Variables|Default|GetAcceleration) (Variables|Default|GetDeceleration)) 0.0 (* _returnvalue_10 (Variables|Default|GetDriftMaxSpeedMultiplier)))))
      (elif (< (Variables|Default|GetCurrentSpeed) _returnvalue_9)
        (Variables|Default|SetCurrentSpeed (Math|Float|Clamp(Float) (+ (Variables|Default|GetCurrentSpeed) (Variables|Default|GetAcceleration) (Variables|Default|GetDeceleration)) 0.0 _returnvalue_9))))
    (elif (> ElapsedSeconds (Variables|Default|GetSecondsToBoost))
      (Variables|Default|SetCurrentSpeed (* (Variables|Default|GetMaxSpeed) (Variables|Default|GetStartupBoost))))))

(event Custom|LookAround
  (params (XVal :type Float%20%28double-precision%29) (YVal :type Float%20%28double-precision%29) (Lock :type Boolean) (Completed :type Boolean))
  (bind _cameraarm (Variables|Default|GetCameraArm))
  (bind _relativerotation (Variables|/Script/Engine.SceneComponent|GetRelativeRotation _cameraarm))
  (Transformation|AddRelativeRotation (Variables|Default|GetCameraArm) (Math|Rotator|MakeRotator 0.0 YVal XVal) false false)
  (Transformation|SetRelativeRotation (Variables|Default|GetCameraArm) (Math|Rotator|MakeRotator (.roll _relativerotation) (Math|Float|ClampAngle (.pitch _relativerotation) -3e+01 0.0) (Math|Float|ClampAngle (.yaw _relativerotation) -2e+01 2e+01)) false false)
  (if (and (not Lock) Completed)
    (Components|MoveComponentTo (Variables|Default|GetCameraArm) (Variables|/Script/Engine.SceneComponent|GetRelativeLocation (Variables|Default|GetCameraArm)) "0, 0, 0" false false 0.2 false :!label _label)
    (else
      (goto _label Stop))))

(event Custom|Turn
  (params (Action%20Value :type Float%20%28double-precision%29) (Completed :type Boolean))
  (if Completed
    (Variables|Default|SetIsTurning false)
    (Variables|Default|SetAttemptToRotateTo 0.0)
    (else
      (Class|Actor|AddActorWorldRotation (Math|Rotator|MakeRotator 0.0 0.0 (* Action%20Value (Variables|Default|GetTurnValue))))
      (Variables|Default|SetIsTurning true)
      (if (Pawn|Components|CharacterMovement|IsWalking (Variables|Character|GetCharacterMovement))
        (Variables|Default|SetAttemptToRotateTo (Math|Float|Clamp(Float) (* Action%20Value (Variables|Default|GetTurnValue) 3e+01) -8e+01 8e+01))))))

(event Custom|ReverseCamera
  (params (Completed :type Boolean) (Toggle :type Boolean))
  (bind _camerareverser (Variables|Default|GetCameraReverser))
  (if (and Completed (not Toggle))
    (Transformation|SetRelativeRotation _camerareverser "0, 0, 0" false false)
    (else
      (Transformation|SetRelativeRotation _camerareverser (Math|Rotator|MakeRotator 0.0 0.0 (Math|Float|%(Float) (+ (.yaw (Variables|/Script/Engine.SceneComponent|GetRelativeRotation (Variables|Default|GetCameraReverser))) 1.8e+02) 3.6e+02)) false false))))

(event Custom|Drift
  (params (Completed :type Boolean))
  (if (not Completed)
    (Variables|Default|SetTurnValue (* (Variables|Default|GetTurnValue) (Variables|Default|GetDriftTurnMultiplier)))
    (Variables|/Script/Engine.CharacterMovementComponent|SetGroundFriction (Variables|Character|GetCharacterMovement) (* (Variables|Default|GetDriftFrictionMultiplier) (Variables|Default|GetFriction)))
    (Variables|Default|SetIsDrifting true)
    (Components|Activation|Activate (Variables|Default|GetNS_Carexhaust) false)
    (else
      (Variables|Default|SetTurnValue (/ (Variables|Default|GetTurnValue) (Variables|Default|GetDriftTurnMultiplier)))
      (Variables|/Script/Engine.CharacterMovementComponent|SetGroundFriction (Variables|Character|GetCharacterMovement) (Variables|Default|GetFriction))
      (Variables|Default|SetIsDrifting false)
      (Components|Activation|Deactivate (Variables|Default|GetNS_Carexhaust)))))

(event Custom|ResetOnStart
  (params (Velocity :type Vector))
  (Pawn|Components|CharacterMovement|SetMovementMode (Variables|Character|GetCharacterMovement) "MOVE_Falling" 0)
  (Physics|AddImpulse (Variables|Character|GetCharacterMovement) Velocity true)
  (Class|AudioComponent|SetPaused (Variables|Default|GetNewVar) false))

(event EventBeginPlay
  (Variables|Default|SetCurrentSpeed 0.0)
  (Variables|/Script/Engine.CharacterMovementComponent|SetGroundFriction (Variables|Character|GetCharacterMovement) (Variables|Default|GetFriction))
  (bind _returnvalue (Audio|CreateSound2D "/Game/Sounds/485355__inspectorj__motor-small-fast-front-04-01-loop.485355__inspectorj__motor-small-fast-front-04-01-loop" 1.0 1.0 0.0 0))
  (bind _output_get (Variables|Default|SetNewVar _returnvalue))
  (Audio|Components|Audio|Play _output_get 0.0)
  (Class|AudioComponent|SetPaused (Variables|Default|GetNewVar) true))

(event EventTick
  (params (DeltaSeconds :type Float%20%28single-precision%29))
  (bind _currentspeed (Variables|Default|GetCurrentSpeed))
  (bind _newvar (Variables|Default|GetNewVar))
  (bind _meshesholder (Variables|Default|GetMeshesHolder))
  (bind _returnvalue (/ _currentspeed 1.2e+02))
  (bind _relativerotation (Variables|/Script/Engine.SceneComponent|GetRelativeRotation _meshesholder))
  (CallFunction|DecelerateandApplySpeed)
  (if (and (> _returnvalue 0.0) (Variables|Default|GetMovable))
    (Audio|Components|Audio|SetPitchMultiplier _newvar _returnvalue)
    (Class|AudioComponent|SetPaused _newvar false)
    (else
      (Class|AudioComponent|SetPaused _newvar true)))
  (Variables|/Script/Engine.SpringArmComponent|SetTargetArmLength (Variables|Default|GetCameraArm) (Math|Interpolation|FInterpTo (Variables|/Script/Engine.SpringArmComponent|GetTargetArmLength (Variables|Default|GetCameraArm)) (Math|Float|Clamp(Float) (* (Math|Vector|VectorLength (Variables|/Script/Engine.MovementComponent|GetVelocity (Variables|Character|GetCharacterMovement))) 0.3) 4e+02 6e+02) (Utilities|Time|GetWorldDeltaSeconds) 1e+01))
  (CallFunction|AttempttoNormalize)
  (Transformation|SetRelativeRotation _meshesholder (Math|Rotator|MakeRotator (Math|Interpolation|FInterpTo (.roll _relativerotation) (Variables|Default|GetAttemptToRotateTo) (Utilities|Time|GetWorldDeltaSeconds) 5.0) (.pitch _relativerotation) (.yaw _relativerotation)) false false))

(event Collision|EventActorBeginOverlap
  (params (OtherActor :type Actor%20Object%20Reference))
  (bind _shipreference (Variables|Default|GetShipReference))
  (if (== (Utilities|GetClass OtherActor) "/Game/Blueprints/BP_SwapToPlane.BP_SwapToPlane_C")
    (Utilities|IsValid _shipreference
      (:Is%20Valid
        (Variables|Default|SetMovable false)
        (Utilities|FlowControl|Delay 0.2)
        (Transformation|SetActorTransform _shipreference (Transformation|GetActorTransform))
        (Rendering|SetActorHiddenInGame true)
        (Rendering|SetActorHiddenInGame _shipreference false)
        (Collision|SetActorEnableCollision _shipreference true)
        (Collision|SetActorEnableCollision false)
        (Default|ResetonStart _shipreference)
        (Pawn|Components|CharacterMovement|DisableMovement (Variables|Character|GetCharacterMovement))))))

(event Input|KeyboardEvents|SpaceBar
  (params (Key :type Key%20Structure :default "None"))
  (bind _ns_boost1 (Variables|Default|GetNS_Boost1))
  (bind _ns_boost2 (Variables|Default|GetNS_Boost2))
  (:Pressed
    (Utilities|FlowControl|DoOnce false :!label _label
      (:Completed
        (Components|Activation|Activate _ns_boost1 false)
        (Components|Activation|Activate _ns_boost2 false)
        (Development|PrintString "Hello"))))
  (:Released
    (Components|Activation|Deactivate _ns_boost1)
    (Components|Activation|Deactivate _ns_boost2)
    (goto _label Reset)))

(fn ConstructionScript)

(fn DecelerateandApplySpeed
  (if (> (Variables|Default|GetCurrentSpeed) 0.0)
    (Variables|Default|SetCurrentSpeed (Math|Float|Clamp(Float) (- (Variables|Default|GetCurrentSpeed) (Variables|Default|GetDeceleration)) 0.0 (Variables|Default|GetCurrentSpeed)))
    (Pawn|Input|AddMovementInput (Transformation|GetActorForwardVector) (* (Variables|Default|GetCurrentSpeed) (Variables|Default|GetSpeedMultiplier) 0.0001) true)))

(fn AttempttoNormalize
  (bind _mesh (Variables|Character|GetMesh))
  (bind _mesh_2 (Variables|Character|GetMesh))
  (bind _capsulecomponent (Variables|Collision|GetCapsuleComponent))
  (bind _returnvalue (Transformation|GetWorldRotation _mesh))
  (bind _returnvalue_2 (Transformation|GetWorldLocation _capsulecomponent))
  (bind _relativerotation (Variables|/Script/Engine.SceneComponent|GetRelativeRotation _mesh_2))
  (bind (_outhit _returnvalue_3) (Class|KismetSystemLibrary|CapsuleTraceSingleforObjects _returnvalue_2 (+ _returnvalue_2 (* (Math|Vector|GetUpVector _capsulecomponent) -2e+02)) 5e+01 5e+01 (Utilities|Array|MakeArray "ObjectTypeQuery1") false 0 "None" true))
  (if _returnvalue_3
    (Transformation|SetWorldRotation (Variables|Character|GetMesh) (Math|Interpolation|RInterpTo _returnvalue (Math|Rotator|MakeRotator (.roll (Math|Rotator|MakeRotfromXZ (Math|Vector|GetForwardVector _mesh) (.ImpactNormal (Collision|BreakHitResult _outhit)))) (.pitch (Class|KismetMathLibrary|MakeRotfromYZ (Math|Vector|GetRightVector _mesh) (.ImpactNormal (Collision|BreakHitResult _outhit)))) (.Yaw (Math|Rotator|BreakRotator _returnvalue))) (Utilities|Time|GetWorldDeltaSeconds) 4e+01) false false)
    (else
      (Transformation|SetRelativeRotation (Variables|Character|GetMesh) (Math|Interpolation|RInterpTo _relativerotation (Math|Rotator|MakeRotator 0.0 0.0 (.Yaw (Math|Rotator|BreakRotator _relativerotation))) (Utilities|Time|GetWorldDeltaSeconds) 1.0) false false))))