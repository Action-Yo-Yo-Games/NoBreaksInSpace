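; Player pawn that spawns a linked car and ship, routing Enhanced Input for driving, drifting, ship movement, boosting, shooting and camera control to them.
; Tick eases the pawn toward the car's camera target, or the ship's when car collision is off, if within range.
; Camera FOV scales with the pawn's velocity.
; Reverse view momentarily zeroes interpolation speed, and P toggles pause.
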(event Custom|Spawn%20Car
  (params (Car%20Type :type Integer) (PlayerID :type Integer))
  (bind _returnvalue (Transformation|GetActorTransform))
  (bind _returnvalue_2 (Game|SpawnActorfromClass "/Game/Blueprints/Player/CarBP/BP_Car.BP_Car_C" (Math|Transform|MakeTransform (Math|Vector|MakeVector (+ (.x (.location _returnvalue)) 1e+02) (.y (.location _returnvalue)) (.z (.location _returnvalue))) (.rotation _returnvalue) (.scale _returnvalue)) "Undefined" "MultiplyWithRoot" 0 0))
  (Variables|Default|SetCar _returnvalue_2)
  (bind _returnvalue_3 (Game|SpawnActorfromClass "/Game/Blueprints/Player/ShipBP/BP_Ship.BP_Ship_C" (Math|Transform|MakeTransform "0.000000,0.000000,-100.000000" "0, 0, 0" "1.000000,1.000000,1.000000") "AlwaysSpawn" "MultiplyWithRoot" 0 0))
  (bind _output_get (Variables|/Game/Blueprints/Player/CarBP/BP_Car.BP_Car_C|SetShipReference (Variables|Default|GetCar) _returnvalue_3))
  (Collision|SetActorEnableCollision _output_get false)
  (Variables|/Game/Blueprints/Player/ShipBP/BP_Ship.BP_Ship_C|SetCarReference _output_get (Variables|Default|GetCar))
  (Default|SetCarType (Variables|Default|GetCar) Car%20Type PlayerID))

(event Input|EnhancedActionEvents|EnhancedInputActionIA_Accelerate
  (params (ActionValue :type Float%20%28double-precision%29) (ElapsedSeconds :type Float%20%28double-precision%29) (TriggeredSeconds :type Float%20%28double-precision%29) (InputAction :type Input%20Action%20Object%20Reference :default "/Game/Blueprints/Player/CarBP/IA_Accelerate.IA_Accelerate"))
  ;[0 0 0] Car Controls
  (Default|Accelerate (Variables|Default|GetCar) ActionValue))

(event Input|EnhancedActionEvents|EnhancedInputActionIA_Boost
  (params (ActionValue :type Float%20%28double-precision%29) (ElapsedSeconds :type Float%20%28double-precision%29) (TriggeredSeconds :type Float%20%28double-precision%29) (InputAction :type Input%20Action%20Object%20Reference :default "/Game/Blueprints/Player/ShipBP/IA_Boost.IA_Boost"))
  (bind _car (Variables|Default|GetCar))
  (bind _shipreference (Variables|/Game/Blueprints/Player/CarBP/BP_Car.BP_Car_C|GetShipReference _car))
  ;[0 0 0] Ship Controls
  (:Started
    (Default|Boost _shipreference false))
  (:Canceled
    (Default|Boost _shipreference true :!label _label))
  (:Completed
    (goto _label)))

(event Input|EnhancedActionEvents|EnhancedInputActionIA_Drift
  (params (ActionValue :type Boolean) (ElapsedSeconds :type Float%20%28double-precision%29) (TriggeredSeconds :type Float%20%28double-precision%29) (InputAction :type Input%20Action%20Object%20Reference :default "/Game/Blueprints/Player/CarBP/IA_Drift.IA_Drift"))
  (bind _car (Variables|Default|GetCar))
  ;[0 0 0] Car Controls
  (:Started
    (Default|Drift _car false))
  (:Canceled
    (Default|Drift _car true :!label _label))
  (:Completed
    (goto _label)))

(event Input|EnhancedActionEvents|EnhancedInputActionIA_Move
  (params (ActionValue :type Vector%202D%20Structure) (ElapsedSeconds :type Float%20%28double-precision%29) (TriggeredSeconds :type Float%20%28double-precision%29) (InputAction :type Input%20Action%20Object%20Reference :default "/Game/Blueprints/Player/ShipBP/IA_Move.IA_Move"))
  (bind _car (Variables|Default|GetCar))
  (bind _shipreference (Variables|/Game/Blueprints/Player/CarBP/BP_Car.BP_Car_C|GetShipReference _car))
  ;[0 0 0] Ship Controls
  (:Triggered
    (Default|Move _shipreference (.x ActionValue) (.y ActionValue) 4e+02 false))
  (:Canceled
    (Default|Move _shipreference (.x ActionValue) (.y ActionValue) 0.0 true :!label _label))
  (:Completed
    (goto _label)))

(event Input|EnhancedActionEvents|EnhancedInputActionIA_ReverseCam
  (params (ActionValue :type Boolean) (ElapsedSeconds :type Float%20%28double-precision%29) (TriggeredSeconds :type Float%20%28double-precision%29) (InputAction :type Input%20Action%20Object%20Reference :default "/Game/Blueprints/Player/CarBP/IA_ReverseCam.IA_ReverseCam"))
  (bind _car (Variables|Default|GetCar))
  (bind _togglereversecam (Variables|Default|GetToggleReverseCam))
  ;[0 0 0] Car Controls
  (:Started
    (Default|ReverseCamera _car false _togglereversecam)
    (Variables|Default|SetInterpSpeed 0.0))
  (:Canceled
    (if (not _togglereversecam) :!label _label
      (Default|ReverseCamera _car true false)
      (Variables|Default|SetInterpSpeed (Variables|Default|GetLag))))
  (:Completed
    (goto _label)))

(event Input|EnhancedActionEvents|EnhancedInputActionIA_LookAround
  (params (ActionValue :type Vector%202D%20Structure) (ElapsedSeconds :type Float%20%28double-precision%29) (TriggeredSeconds :type Float%20%28double-precision%29) (InputAction :type Input%20Action%20Object%20Reference :default "/Game/Blueprints/Player/CarBP/IA_LookAround.IA_LookAround"))
  (bind _car (Variables|Default|GetCar))
  (bind _lockcameramovements (Variables|Default|GetLockCameraMovements))
  ;[0 0 0] Car Controls
  (:Triggered
    (Default|LookAround _car (.x ActionValue) (.y ActionValue) _lockcameramovements false))
  (:Canceled
    (Default|LookAround _car (.x ActionValue) (.y ActionValue) _lockcameramovements true :!label _label))
  (:Completed
    (goto _label)))

(event Input|EnhancedActionEvents|EnhancedInputActionIA_Shoot
  (params (ActionValue :type Boolean) (ElapsedSeconds :type Float%20%28double-precision%29) (TriggeredSeconds :type Float%20%28double-precision%29) (InputAction :type Input%20Action%20Object%20Reference :default "/Game/Blueprints/Player/ShipBP/IA_Shoot.IA_Shoot"))
  (bind _car (Variables|Default|GetCar))
  (bind _shipreference (Variables|/Game/Blueprints/Player/CarBP/BP_Car.BP_Car_C|GetShipReference _car))
  ;[0 0 0] Ship Controls
  (:Triggered
    (Default|Shoot _shipreference false))
  (:Canceled
    (Default|Shoot _shipreference true :!label _label))
  (:Completed
    (goto _label)))

(event Input|EnhancedActionEvents|EnhancedInputActionIA_Turn
  (params (ActionValue :type Float%20%28double-precision%29) (ElapsedSeconds :type Float%20%28double-precision%29) (TriggeredSeconds :type Float%20%28double-precision%29) (InputAction :type Input%20Action%20Object%20Reference :default "/Game/Blueprints/Player/CarBP/IA_Turn.IA_Turn"))
  (bind _car (Variables|Default|GetCar))
  ;[0 0 0] Car Controls
  (:Triggered
    (Default|Turn _car ActionValue false))
  (:Canceled
    (Default|Turn _car ActionValue true :!label _label))
  (:Completed
    (goto _label)))

(event EventBeginPlay
  (CallFunction|SpawnCar (Variables|Default|GetCarType) (Variables|Default|GetPlayerID))
  (bind _asplayer_controller (Utilities|Casting|CastToPlayerController (Pawn|GetController))
    (:then
      (Utilities|IsValid (PlayerController|LocalPlayerSubsystems|GetEnhancedInputLocalPlayerSubsystem _asplayer_controller)
        (:Is%20Valid
          (Input|AddMappingContext (PlayerController|LocalPlayerSubsystems|GetEnhancedInputLocalPlayerSubsystem _asplayer_controller) "/Game/Blueprints/Player/IMC_Player.IMC_Player" 0 "(bIgnoreAllPressedKeysUntilRelease=True,bForceImmediately=False,bNotifyUserSettings=False)"))
        (:Is%20Not%20Valid
          (Development|PrintString "ControllerInvalid"))))
    (:CastFailed
      (Development|PrintString "CastFail"))))

(event EventTick
  (params (DeltaSeconds :type Float%20%28single-precision%29))
  (if (Collision|GetActorEnableCollision (Variables|Default|GetCar))
    (Variables|Default|SetCameraTarget (Variables|/Game/Blueprints/Player/CarBP/BP_Car.BP_Car_C|GetCameraTarget (Variables|Default|GetCar)))
    (else
      (Variables|Default|SetCameraTarget (Variables|/Game/Blueprints/Player/ShipBP/BP_Ship.BP_Ship_C|GetCameraTarget (Variables|/Game/Blueprints/Player/CarBP/BP_Car.BP_Car_C|GetShipReference (Variables|Default|GetCar))))))
  (if (< (Math|Vector|Distance(Vector) (Transformation|GetWorldLocation (Variables|Default|GetCameraTarget)) (Transformation|GetActorLocation)) 5e+03)
    (Transformation|SetActorLocationAndRotation (Math|Interpolation|VInterpTo (Transformation|GetActorLocation) (Transformation|GetWorldLocation (Variables|Default|GetCameraTarget)) (Utilities|Time|GetWorldDeltaSeconds) (Variables|Default|GetInterpSpeed)) (Math|Interpolation|RInterpTo (Transformation|GetActorRotation) (Transformation|GetWorldRotation (Variables|Default|GetCameraTarget)) (Utilities|Time|GetWorldDeltaSeconds) (Variables|Default|GetInterpSpeed)))
    (Camera|SetFieldOfView (Variables|Default|GetCamera) (Math|Interpolation|FInterpTo (Variables|/Script/Engine.CameraComponent|GetFieldOfView (Variables|Default|GetCamera)) (Math|Float|Clamp(Float) (* (Math|Vector|VectorLength (Transformation|GetVelocity)) 0.05) 9e+01 1.4e+02) (Utilities|Time|GetWorldDeltaSeconds) 1e+01))
    (Variables|Default|SetInterpSpeed (Variables|Default|GetLag))))

(event Input|KeyboardEvents|P
  (params (Key :type Key%20Structure :default "None"))
  ;[1 1 1] Pause menu
  (:Pressed
    (if (Variables|Default|GetIsPaused)
      (Game|SetGamePaused false)
      (Variables|Default|SetIsPaused false)
      (else
        (Game|SetGamePaused true)
        (Variables|Default|SetIsPaused true)))))

(fn ConstructionScript)